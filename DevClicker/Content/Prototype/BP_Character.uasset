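; Player Blueprint for an idle clicker prototype, handling currency, clicks, saving and ad prompts.
; BeginPlay checks slot "Save1" but loads "testSave", or creates a save, then builds the HUD and starts looping income and ad-popup timers.
; Offline earnings come from time since LastOpened, without the multiplier, on launch and foregrounding; backgrounding stamps the time and saves.
; Clicks add currency, using a retriggerable delay to end sound and HUD feedback.
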(event Custom|GameUpdate
  (bind _savegame (Variables|Default|GetSaveGame))
  (bind _savegame_2 (Variables|Default|GetSaveGame))
  (bind _earnings_per_seconds (Variables|/Game/Prototype/Data/BP_SaveGame.BP_SaveGame_C|GetEarnings%20Per%20seconds _savegame_2))
  (bind _earnings_per_seconds_2 (Variables|/Game/Prototype/Data/BP_SaveGame.BP_SaveGame_C|GetEarnings%20Per%20seconds _savegame))
  ;[1 1 1] update UI and increase the amount of currency the player owns
  (Default|UpdateUI (Variables|Default|GetHUD) (Variables|/Game/Prototype/Data/BP_SaveGame.BP_SaveGame_C|Getcurrency (Variables|Default|GetSaveGame)) (+ _earnings_per_seconds_2 (* _earnings_per_seconds_2 (Variables|/Game/Prototype/Data/BP_SaveGame.BP_SaveGame_C|GetCurrencyMultiplier _savegame))))
  (Variables|/Game/Prototype/Data/BP_SaveGame.BP_SaveGame_C|Setcurrency _savegame_2 (+ (Variables|/Game/Prototype/Data/BP_SaveGame.BP_SaveGame_C|Getcurrency _savegame_2) (/ (+ _earnings_per_seconds (* _earnings_per_seconds (Variables|/Game/Prototype/Data/BP_SaveGame.BP_SaveGame_C|GetCurrencyMultiplier _savegame_2))) (Variables|Default|Getadjustment%20from%20ticks%20to%20seconds)))))

(event Custom|save
  (bind _savegame (Variables|Default|GetSaveGame))
  ;[1 1 1] Save the game
  (SaveGame|SaveGametoSlot _savegame (Variables|/Game/Prototype/Data/BP_SaveGame.BP_SaveGame_C|GetSaveName _savegame) (Variables|/Game/Prototype/Data/BP_SaveGame.BP_SaveGame_C|GetUserIndex _savegame)))

(event Custom|ApplicationHasEnteredForegroundDelegate_Event
  ;[1 1 1] Setup events for when the player puts the game into the background or comes back from this
  (CallFunction|CalculateIdleEarnings))

(event Custom|Calculate%20idle%20earnings
  ;[1 1 1] calculate idle earnings
  ;;[1 1 1] calculate how long its been since the game was last opened
  (Development|PrintString (Utilities|String|ToString(Integer) (.minutes (- (Math|DateTime|Now) (Variables|/Game/Prototype/Data/BP_SaveGame.BP_SaveGame_C|GetLastOpened (Variables|Default|GetSaveGame))))))
  (Development|PrintString (Utilities|String|ToString(Integer) (.seconds (- (Math|DateTime|Now) (Variables|/Game/Prototype/Data/BP_SaveGame.BP_SaveGame_C|GetLastOpened (Variables|Default|GetSaveGame))))))
  (Variables|/Game/Prototype/Data/BP_SaveGame.BP_SaveGame_C|Setcurrency (Variables|Default|GetSaveGame) (+ (* (Variables|/Game/Prototype/Data/BP_SaveGame.BP_SaveGame_C|GetEarnings%20Per%20seconds (Variables|Default|GetSaveGame)) (+ (* (.days (- (Math|DateTime|Now) (Variables|/Game/Prototype/Data/BP_SaveGame.BP_SaveGame_C|GetLastOpened (Variables|Default|GetSaveGame)))) (Variables|Default|GetSecondsInADay)) (* (.hours (- (Math|DateTime|Now) (Variables|/Game/Prototype/Data/BP_SaveGame.BP_SaveGame_C|GetLastOpened (Variables|Default|GetSaveGame)))) (Variables|Default|GetSecondsInAnHour)) (.seconds (- (Math|DateTime|Now) (Variables|/Game/Prototype/Data/BP_SaveGame.BP_SaveGame_C|GetLastOpened (Variables|Default|GetSaveGame)))) (* (.minutes (- (Math|DateTime|Now) (Variables|/Game/Prototype/Data/BP_SaveGame.BP_SaveGame_C|GetLastOpened (Variables|Default|GetSaveGame)))) (Variables|Default|GetSecondsInAMinute)))) (Variables|/Game/Prototype/Data/BP_SaveGame.BP_SaveGame_C|Getcurrency (Variables|Default|GetSaveGame))))
  (Variables|/Game/Prototype/Data/BP_SaveGame.BP_SaveGame_C|SetLastOpened (Variables|Default|GetSaveGame) (Math|DateTime|Now)))

(event Custom|ApplicationWillEnterBackground
  ;[1 1 1] When the player exits the game, save their progress
  (Variables|/Game/Prototype/Data/BP_SaveGame.BP_SaveGame_C|SetLastOpened (Variables|Default|GetSaveGame) (Math|DateTime|Now))
  (CallFunction|Save))

(event Custom|Suggest%20Ad
  (bind _hud (Variables|Default|GetHUD))
  ;[1 1 1] make ad notification popup appear every 6 minutes
  (Widget|SetVisibility (Variables|/Game/UI/WBP_HUD.WBP_HUD_C|GetWBP_adInGameNotif _hud) "Visible")
  (Default|PopupActive (Variables|/Game/UI/WBP_HUD.WBP_HUD_C|GetWBP_adPopup _hud)))

(event EventBeginPlay
  ;[1 1 1] ensure a save exists
  (bind _returnvalue (SaveGame|DoesSaveGameExist "Save1"))
  (if _returnvalue
    (bind _returnvalue_2 (SaveGame|LoadGamefromSlot "testSave"))
    (bind _asbp_save_game (Utilities|Casting|CastToBP_SaveGame _returnvalue_2))
    (Variables|Default|SetSaveGame _asbp_save_game)
    (else
      (bind _returnvalue_3 (SaveGame|CreateSaveGameObject "/Game/Prototype/Data/BP_SaveGame.BP_SaveGame_C"))
      (Variables|Default|SetSaveGame _returnvalue_3)))
  ;[1 1 1] create HUD widget
  (bind _returnvalue_4 (UserInterface|CreateWidget "/Game/UI/WBP_HUD.WBP_HUD_C" (Game|GetPlayerController 0)))
  (bind _output_get (Variables|Default|SetHUD _returnvalue_4))
  (UserInterface|Viewport|AddtoViewport _output_get 0)
  (Default|Init (Variables|Default|GetHUD) (Variables|/Game/Prototype/Data/BP_SaveGame.BP_SaveGame_C|Getcurrency (Variables|Default|GetSaveGame)) (Variables|Default|GetSaveGame) self)
  (Utilities|Time|SetTimerbyEvent (delegate Custom|GameUpdate) 0.1 true true)
  (CallFunction|CalculateIdleEarnings)
  ;[1 1 1] Setup events for when the player puts the game into the background or comes back from this
  (bind _returnvalue_5 (AddComponent|AddApplicationLifecycleComponent))
  (bind _output_get_2 (Variables|Default|SetapplicationLifeCycle _returnvalue_5))
  (CallFunction|Save)
  (EventDispatchers|BindEventtoApplicationWillEnterBackgroundDelegate _output_get_2 (delegate Custom|ApplicationWillEnterBackground))
  (EventDispatchers|AssignApplicationHasEnteredForegroundDelegate (Variables|Default|GetapplicationLifeCycle) (delegate Custom|ApplicationHasEnteredForegroundDelegate_Event))
  ;[1 1 1] make ad notification popup appear every 6 minutes
  (Utilities|Time|SetTimerbyEvent (delegate Custom|Suggest%20Ad) 3e+02 true))

(event EventNewFunction
  (bind _clicksound (Variables|Default|GetClickSound))
  (bind _savegame (Variables|Default|GetSaveGame))
  ;[1 1 1] player clicked
  ;;[1 1 1] click space clicked to earn money
  (Default|Clicking (Variables|Default|GetHUD))
  (Variables|/Game/Prototype/Data/BP_SaveGame.BP_SaveGame_C|Setcurrency (Variables|Default|GetSaveGame) (+ (Variables|/Game/Prototype/Data/BP_SaveGame.BP_SaveGame_C|GetClick%20Amount%20Increase _savegame) (Variables|/Game/Prototype/Data/BP_SaveGame.BP_SaveGame_C|Getcurrency _savegame)))
  ;;[1 1 1] handle playing of the click SFX (prevent it from overlapping)
  (if (Audio|Components|Audio|IsPlaying _clicksound)
    _
    (else
      (Audio|Components|Audio|Play _clicksound 0.0)))
  (Utilities|FlowControl|RetriggerableDelay 1.0)
  (Audio|Components|Audio|Stop (Variables|Default|GetClickSound))
  (Default|NotClicking (Variables|Default|GetHUD)))

(fn ConstructionScript)