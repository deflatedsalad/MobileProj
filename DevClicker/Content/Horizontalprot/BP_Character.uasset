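; Player character for an idle clicker game, owning the currency loop, the HUD and the save game.
; On begin play it loads or creates the save, creates the HUD and credits offline earnings from the time elapsed since LastOpened.
; A looping timer adds passive income and refreshes the HUD.
; Clicks add currency, save, and use a retriggerable delay to end click audio and HUD feedback once clicking pauses.
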(event Custom|GameUpdate
  (bind _savegame (Variables|Default|GetSaveGame))
  ;[1 1 1] update UI and increase the amount of currency the player owns
  (Default|UpdateUI (Variables|Default|GetHUD) (stale EventNewFunction _output_get))
  (Variables|/Game/Horizontalprot/Data/BP_SaveGame.BP_SaveGame_C|Setcurrency _savegame (+ (Variables|/Game/Horizontalprot/Data/BP_SaveGame.BP_SaveGame_C|Getcurrency _savegame) (/ (Variables|/Game/Horizontalprot/Data/BP_SaveGame.BP_SaveGame_C|GetEarnings%20Per%20seconds _savegame) (Variables|Default|Getadjustment%20from%20ticks%20to%20seconds)))))

(event Custom|save
  (bind _savegame (Variables|Default|GetSaveGame))
  (bind _returnvalue (SaveGame|SaveGametoSlot _savegame (Variables|/Game/Horizontalprot/Data/BP_SaveGame.BP_SaveGame_C|GetSaveName _savegame) (Variables|/Game/Horizontalprot/Data/BP_SaveGame.BP_SaveGame_C|GetUserIndex _savegame))))

(event EventBeginPlay
  (bind _returnvalue (SaveGame|DoesSaveGameExist "testSave"))
  (if _returnvalue
    (bind _returnvalue_2 (SaveGame|LoadGamefromSlot "testSave"))
    (bind _asbp_save_game (Utilities|Casting|CastToBP_SaveGame _returnvalue_2))
    (Variables|Default|SetSaveGame _asbp_save_game)
    (else
      (bind _returnvalue_3 (SaveGame|CreateSaveGameObject "/Game/Horizontalprot/Data/BP_SaveGame.BP_SaveGame_C"))
      (Variables|Default|SetSaveGame _returnvalue_3)))
  (bind _returnvalue_4 (UserInterface|CreateWidget "/Game/UI/WBP_HUD.WBP_HUD_C" (Game|GetPlayerController 0)))
  (bind _output_get (Variables|Default|SetHUD _returnvalue_4))
  (UserInterface|Viewport|AddtoViewport _output_get 0)
  (Utilities|Time|SetTimerbyEvent (delegate Custom|GameUpdate) 0.1 true true)
  (Default|Init (Variables|Default|GetHUD) (Variables|/Game/Horizontalprot/Data/BP_SaveGame.BP_SaveGame_C|Getcurrency (Variables|Default|GetSaveGame)) (Variables|Default|GetSaveGame) self)
  ;[1 1 1] calculate how long its been since the game was last opened
  (Development|PrintString (Utilities|String|ToString(Integer) (.minutes (- (Math|DateTime|Now) (Variables|/Game/Horizontalprot/Data/BP_SaveGame.BP_SaveGame_C|GetLastOpened (Variables|Default|GetSaveGame))))))
  (Development|PrintString (Utilities|String|ToString(Integer) (.seconds (- (Math|DateTime|Now) (Variables|/Game/Horizontalprot/Data/BP_SaveGame.BP_SaveGame_C|GetLastOpened (Variables|Default|GetSaveGame))))))
  (Variables|/Game/Horizontalprot/Data/BP_SaveGame.BP_SaveGame_C|Setcurrency (Variables|Default|GetSaveGame) (+ (* (Variables|/Game/Horizontalprot/Data/BP_SaveGame.BP_SaveGame_C|GetEarnings%20Per%20seconds (Variables|Default|GetSaveGame)) (+ (* (.days (- (Math|DateTime|Now) (Variables|/Game/Horizontalprot/Data/BP_SaveGame.BP_SaveGame_C|GetLastOpened (Variables|Default|GetSaveGame)))) (Variables|Default|GetSecondsInADay)) (* (.hours (- (Math|DateTime|Now) (Variables|/Game/Horizontalprot/Data/BP_SaveGame.BP_SaveGame_C|GetLastOpened (Variables|Default|GetSaveGame)))) (Variables|Default|GetSecondsInAnHour)) (.seconds (- (Math|DateTime|Now) (Variables|/Game/Horizontalprot/Data/BP_SaveGame.BP_SaveGame_C|GetLastOpened (Variables|Default|GetSaveGame)))) (* (.minutes (- (Math|DateTime|Now) (Variables|/Game/Horizontalprot/Data/BP_SaveGame.BP_SaveGame_C|GetLastOpened (Variables|Default|GetSaveGame)))) (Variables|Default|GetSecondsInAMinute)))) (Variables|/Game/Horizontalprot/Data/BP_SaveGame.BP_SaveGame_C|Getcurrency (Variables|Default|GetSaveGame))))
  (Variables|/Game/Horizontalprot/Data/BP_SaveGame.BP_SaveGame_C|SetLastOpened (Variables|Default|GetSaveGame) (Math|DateTime|Now))
  (CallFunction|Save))

(event EventEndPlay
  (params (EndPlayReason :type EEndPlayReason%20Enum :default "Destroyed"))
  (Variables|/Game/Horizontalprot/Data/BP_SaveGame.BP_SaveGame_C|SetLastOpened (Variables|Default|GetSaveGame) (Math|DateTime|Now))
  (CallFunction|Save))

(event EventNewFunction
  (bind _clicksound (Variables|Default|GetClickSound))
  ;[1 1 1] click space clicked to earn money
  (Default|Clicking (Variables|Default|GetHUD))
  (bind _output_get (Variables|/Game/Horizontalprot/Data/BP_SaveGame.BP_SaveGame_C|Setcurrency (Variables|Default|GetSaveGame) (+ (Variables|Default|GetClickAddAmount) (Variables|/Game/Horizontalprot/Data/BP_SaveGame.BP_SaveGame_C|Getcurrency (Variables|Default|GetSaveGame)))))
  (CallFunction|Save)
  (if (Audio|Components|Audio|IsPlaying _clicksound)
    _
    (else
      (Audio|Components|Audio|Play _clicksound 0.0)))
  (Utilities|FlowControl|RetriggerableDelay 1.0)
  (Development|PrintString "timer ended")
  (Audio|Components|Audio|Stop (Variables|Default|GetClickSound))
  (Audio|PlaySound2D "/Game/SFX/Keyboard/keyboard_end.keyboard_end" 1.0 1.0 0.0 0 0)
  (Default|NotClicking (Variables|Default|GetHUD)))

(fn ConstructionScript)